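; Openable door actor that swings open and closed in response to open and close requests from its OpenDoor component.
; BeginPlay caches the initial rotation and location, and a timeline drives a yaw offset combined with that starting rotation.
; Open plays the timeline and close reverses it, while a timeline event track plays a creak sound at the cached location.
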(event `self.ReceiveBeginPlay`
  (set `self.InitialRotation` (`self.K2_GetActorRotation`))
  (set `self.Initial Location` (`self.K2_GetActorLocation`)))

(event `self.OpenDoor.OnOpenRequest`
  (bind (_direction _openangle) (`Timeline|Timeline_0` :!label _label)
    (:`Update`
      (`self.K2_SetActorRotation` (`KismetMathLibrary.ComposeRotators` (`self.InitialRotation`) (`KismetMathLibrary.MakeRotator` 0.0 0.0 _openangle))))
    (:`SoundTiming`
      (`GameplayStatics.PlaySoundAtLocation` "/Game/Audio/DoorCreak.DoorCreak" (`self.Initial Location`)))))

(event `self.OpenDoor.OnCloseRequest`
  (goto _label :!via `Reverse`))

(fn `UserConstructionScript`)